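; BP_PNJ is an interactable NPC that shows text and takes over the camera when the player interacts with it.
; Its text render starts hidden, and each Interract event alternates through a FlipFlop between showing it while blending the view to the NPC, and hiding it while blending back to the controlled pawn.
; Exiting sets ShouldMove true on the top-down controller, but the node that sets it false is unconnected.
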(event EventBeginPlay
  (Rendering|SetVisibility (Variables|Default|GetTextRender1) false false))

(event Collision|EventActorBeginOverlap
  (params (OtherActor :type Actor%20Object%20Reference)))

(event EventTick
  (params (DeltaSeconds :type Float%20%28single-precision%29)))

(event EventInterract
  (bind _playercontroller (CallFunction|GetTopDownController))
  (Utilities|FlowControl|FlipFlop
    (:A
      (Rendering|SetVisibility (Variables|Default|GetTextRender1) true false)
      (Game|Player|SetViewTargetwithBlend (CallFunction|GetTopDownController) self 1.0 "VTBlend_Linear" 1.0 false))
    (:B
      (Rendering|SetVisibility (Variables|Default|GetTextRender1) false false)
      (Game|Player|SetViewTargetwithBlend _playercontroller (Pawn|GetControlledPawn _playercontroller) 1.0 "VTBlend_Linear" 0.0 false)
      (Variables|/Game/TopDown/Blueprints/BP_TopDownController.BP_TopDownController_C|SetShouldMove _playercontroller true))))

(fn ConstructionScript)